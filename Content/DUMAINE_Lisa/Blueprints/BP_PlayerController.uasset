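; BP_PlayerController is a player controller that tracks the player's health and handles death.
; GetHealed and GetDammage adjust HPPlayer and print the new value on screen.
; When damage brings health to zero or below, GetDead moves the third-person character to a hardcoded location, prints a French death message and resets health to a fixed value.
; BeginPlay and Tick are unused, so all logic runs through these functions.
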(event EventBeginPlay)

(event EventTick
  (params (DeltaSeconds :type Float%20%28single-precision%29)))

(fn ConstructionScript)

(fn GetHealed
  (params (ValueHeal :type Integer))
  (bind _output_get (Variables|Default|SetHP_Player (+ ValueHeal (Variables|Default|GetHP_Player))))
  (Development|PrintString (Utilities|String|ToString(Integer) _output_get))
  (Development|PrintString "Hp Player :"))

(fn GetDammage
  (params (Dammage :type Integer))
  (bind _output_get (Variables|Default|SetHP_Player (- (Variables|Default|GetHP_Player) Dammage)))
  (Development|PrintString (Utilities|String|ToString(Integer) _output_get))
  (Development|PrintString "Hp Player :")
  (if (>= 0 (Variables|Default|GetHP_Player))
    (CallFunction|GetDead)))

(fn GetDead
  (bind _asbp_third_person_character (Utilities|Casting|CastToBP_ThirdPersonCharacter (Game|GetPlayerCharacter 0)))
  (Transformation|SetActorLocation _asbp_third_person_character "900.000000,100.000000,92.000000" false false)
  (Development|PrintString "T'es mort")
  (Variables|Default|SetHP_Player 20))